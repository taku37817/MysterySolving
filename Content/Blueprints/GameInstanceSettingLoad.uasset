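; Game instance Blueprint that initializes the graphics settings widget when the game instance starts.
; On Init it creates WBP_Setting_WBP, stores the reference, adds it to the viewport if not visible, and copies its GraphicsQualityLevel into the widget.
; UpdateGraphicsText then maps that level to a Low, Middle or High label on the widget.
; It only sets the widget's value and text, without loading saved data or applying engine quality settings.
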(event `self.ReceiveInit`
  (`self.GraphicSettingLadeInit`))

(event `GraphicSettingLadeInit`
  (bind _returnvalue (`|CreateWidget` "/Game/WidgetBlueprint/WBP_Setting_WBP.WBP_Setting_WBP_C"))
  (bind _output_get (set `self.WBP_Setting_WBP` _returnvalue))
  (if (not (`Widget.IsVisible` _output_get))
    (`UserWidget.AddToViewport` _output_get 0))
  (set `/Game/WidgetBlueprint/WBP_Setting_WBP.GraphicsQualityLevel` (`self.GraphicsQualityLevel`) _output_get)
  (`self.UpdateGraphicsText`))

(fn `UpdateGraphicsText`
  (`TextBlock.SetText` (`/Game/WidgetBlueprint/WBP_Setting_WBP.Text_SettingValue` (`self.WBP_Setting_WBP`)) (select `int` (`self.GraphicsQualityLevel`) :`0` "Low" :`1` "Middle" :`2` "High")))