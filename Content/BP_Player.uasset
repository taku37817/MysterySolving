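; Player Blueprint for a key-and-door game, handling the HUD widgets and the grab, door and pause inputs.
; BeginPlay creates hidden key icon, message and game-over widgets, loads user settings and sets countdown variables.
; Tick polls the Grabber's per-key flags to show or hide silver, gold and brown pickup messages.
; Inputs toggle Grabber grab/release, hold DoorKeyManager's open-door flag, and drive GameMode_Pause while syncing GameMode_GameOver's pause flag.
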(event `self.ReceiveBeginPlay`
  (`self.Garbbed Message Gargoyle Begine Play`)
  (`self.TimerSetBeginPlay`)
  (`self.SilverKeyMessageBeginePlay`)
  (`self.GoldKeyMessageBeginePlay`)
  (`self.BrownKeyMessageBeginePlay`)
  (`self.SilverKeyImageBeginePlay`)
  (`self.GoldKeyImageBeginePlay`)
  (`self.BronzeKeyImageBeginePlay`)
  (`self.GameOverBeginePlay`)
  (`self.SettingLoadBeginPlay`)
  (`self.SilverKeyNotHavMeessageBeginPlay`)
  (`self.HaveKey_Message`))

(event `Garbbed Message Gargoyle Begine Play`)

(event `SilverKeyImageBeginePlay`
  (bind _returnvalue (`|CreateWidget` "/Game/WidgetBlueprint/SilverKey.SilverKey_C"))
  (bind _output_get (set `self.WBP_SilverKey` _returnvalue))
  (`UserWidget.AddToViewport` _output_get 0)
  (`Widget.SetVisibility` _output_get "Hidden"))

(event `GoldKeyImageBeginePlay`
  (bind _returnvalue (`|CreateWidget` "/Game/WidgetBlueprint/GoldKey.GoldKey_C"))
  (bind _output_get (set `self.WBP_GoldKey` _returnvalue))
  (`UserWidget.AddToViewport` _output_get 0)
  (`Widget.SetVisibility` _output_get "Hidden"))

(event `BronzeKeyImageBeginePlay`
  (bind _returnvalue (`|CreateWidget` "/Game/WidgetBlueprint/BrownKey.BrownKey_C"))
  (bind _output_get (set `self.WBP_BrownKey` _returnvalue))
  (`UserWidget.AddToViewport` _output_get 0)
  (`Widget.SetVisibility` _output_get "Hidden"))

(event `SilverKeyMessageBeginePlay`
  (bind _returnvalue (`|CreateWidget` "/Game/WidgetBlueprint/WBP_Silver_Grabbed_Message.WBP_Silver_Grabbed_Message_C"))
  (bind _output_get (set `self.WBP_Silver_Grabbed_Message` _returnvalue))
  (`UserWidget.AddToViewport` _output_get 0)
  (`Widget.SetVisibility` _output_get "Hidden"))

(event `GameOverBeginePlay`
  (bind _returnvalue (`|CreateWidget` "/Game/WidgetBlueprint/WBP_GameOverWidget.WBP_GameOverWidget_C"))
  (bind _output_get (set `self.WBP_GameOver` _returnvalue))
  (`UserWidget.AddToViewport` _output_get 0)
  (`Widget.SetVisibility` _output_get "Hidden"))

(event `GoldKeyMessageBeginePlay`
  (bind _returnvalue (`|CreateWidget` "/Game/WidgetBlueprint/WBP_Gold_Grabbed_Message.WBP_Gold_Grabbed_Message_C"))
  (bind _output_get (set `self.WBP_Gold_Grabbed_Message` _returnvalue))
  (`UserWidget.AddToViewport` _output_get 0)
  (`Widget.SetVisibility` _output_get "Hidden"))

(event `CountdownBeginPlay`
  (bind _returnvalue (`|CreateWidget` "/Game/WidgetBlueprint/WBP_Countdown.WBP_Countdown_C"))
  (bind _output_get (set `self.WBP_Countdown` _returnvalue))
  (`UserWidget.AddToViewport` _output_get 0)
  (`Widget.SetVisibility` _output_get "Visible"))

(event `BrownKeyMessageBeginePlay`
  (bind _returnvalue (`|CreateWidget` "/Game/WidgetBlueprint/WBP_Brown_Grabbed_Message.WBP_Brown_Grabbed_Message_C"))
  (bind _output_get (set `self.WBP_Brown_Grabbed_Message` _returnvalue))
  (`UserWidget.AddToViewport` _output_get 0)
  (`Widget.SetVisibility` _output_get "Hidden"))

(event `SilverKeyNotHavMeessageBeginPlay`
  (bind _returnvalue (`|CreateWidget` "/Game/WidgetBlueprint/WBP_Not_HaveKey_Message.WBP_Not_HaveKey_Message_C"))
  (bind _output_get (set `self.WBP_Not_HaveKey_Message` _returnvalue))
  (`UserWidget.AddToViewport` _output_get 0)
  (`Widget.SetVisibility` _output_get "Hidden"))

(event `SettingLoadBeginPlay`
  (bind _returnvalue (`GameUserSettings.GetGameUserSettings`))
  (`GameUserSettings.LoadSettings` _returnvalue false)
  (`GameUserSettings.ApplySettings` _returnvalue true))

(event `HaveKey_Message`
  (bind _returnvalue (`|CreateWidget` "/Game/WidgetBlueprint/WBP_HaveKey_Message.WBP_HaveKey_Message_C"))
  (bind _output_get (set `self.WBP_HaveKey_Message` _returnvalue))
  (`UserWidget.AddToViewport` _output_get 0)
  (`Widget.SetVisibility` _output_get "Hidden"))

(event `TimerSetBeginPlay`
  (set `self.CountDownTime` 2.0)
  (set `self.bIsConutingDown` true))

(event `self.ReceiveTick`
  (params (DeltaSeconds :type "Float (single-precision)"))
  (`self.SilverKeyGrabbedMessageTick`)
  (`self.GoldKeyGrabbedMessageTick`)
  (`self.BrownKeyGrabbedMessageTick`))

(event `SilverKeyGrabbedMessageTick`
  (bind _wbp_silver_grabbed_message (`self.WBP_Silver_Grabbed_Message`))
  (if (`|GetArrayItem` (`Grabber.bIsKeyGrabbedMessage` (`self.Grabber`)))
    (bind _output_get (set `self.WBP_Silver_Grabbed_Message` _wbp_silver_grabbed_message))
    (if (not (`Widget.IsInViewport` _output_get))
      (`UserWidget.AddToViewport` _output_get 0))
    (`Widget.SetVisibility` _output_get "Visible")
    (else
      (bind _output_get_2 (set `self.WBP_Silver_Grabbed_Message` _wbp_silver_grabbed_message))
      (if (not (`Widget.IsInViewport` _output_get_2))
        (`UserWidget.AddToViewport` _output_get_2 0))
      (`Widget.SetVisibility` _output_get_2 "Hidden"))))

(event `GoldKeyGrabbedMessageTick`
  (bind _wbp_gold_grabbed_message (`self.WBP_Gold_Grabbed_Message`))
  (if (`|GetArrayItem` (`Grabber.bIsKeyGrabbedMessage` (`self.Grabber`)) 1)
    (bind _output_get (set `self.WBP_Gold_Grabbed_Message` _wbp_gold_grabbed_message))
    (if (not (`Widget.IsInViewport` _output_get))
      (`UserWidget.AddToViewport` _output_get 0))
    (`Widget.SetVisibility` _output_get "Visible")
    (else
      (bind _output_get_2 (set `self.WBP_Gold_Grabbed_Message` _wbp_gold_grabbed_message))
      (if (not (`Widget.IsInViewport` _output_get_2))
        (`UserWidget.AddToViewport` _output_get_2 0))
      (`Widget.SetVisibility` _output_get_2 "Hidden"))))

(event `BrownKeyGrabbedMessageTick`
  (bind _wbp_brown_grabbed_message (`self.WBP_Brown_Grabbed_Message`))
  (if (`|GetArrayItem` (`Grabber.bIsKeyGrabbedMessage` (`self.Grabber`)) 2)
    (bind _output_get (set `self.WBP_Brown_Grabbed_Message` _wbp_brown_grabbed_message))
    (if (not (`Widget.IsInViewport` _output_get))
      (`UserWidget.AddToViewport` _output_get 0))
    (`Widget.SetVisibility` _output_get "Visible")
    (else
      (bind _output_get_2 (set `self.WBP_Brown_Grabbed_Message` _wbp_brown_grabbed_message))
      (if (not (`Widget.IsInViewport` _output_get_2))
        (`UserWidget.AddToViewport` _output_get_2 0))
      (`Widget.SetVisibility` _output_get_2 "Hidden"))))

(event `InputAction|Grab`
  (params (Key :type "Key Structure"))
  (:`Pressed`
    (`self.InputAction Grabbed`)))

(event `InputAction Grabbed`
  (bind _grabber (`self.Grabber`))
  (if (`self.IsGrabbing`)
    (`Grabber.Grab` _grabber)
    (set `self.IsGrabbing` false)
    (else
      (`Grabber.Release` _grabber)
      (set `self.IsGrabbing` true))))

(event `InputAction|RightClickAction`
  (params (Key :type "Key Structure"))
  (bind _doorkeymanager (`self.DoorKeyManager`))
  (:`Pressed`
    (set `DoorKeyManager.isOpenDoor` true _doorkeymanager))
  (:`Released`
    (set `DoorKeyManager.isOpenDoor` false _doorkeymanager)))

(event `InputAction|PauseButton`
  (params (Key :type "Key Structure"))
  (:`Pressed`
    (`self.IsPauseJudge_PauseButton`)
    (`self.PauseButtonAction`)))

(event `PauseButtonAction`
  (bind _returnvalue (`GameplayStatics.GetActorOfClass` "/Script/MysterySolving.GameMode_Pause"))
  (bind _output_get (set `self.GameMode_Pause` _returnvalue))
  (`GameMode_Pause.Pause` _output_get))

(event `IsPauseJudge_PauseButton`
  (bind _returnvalue (`GameplayStatics.GetActorOfClass` "/Script/MysterySolving.GameMode_GameOver"))
  (bind _output_get (set `self.GameMode_GameOver` _returnvalue))
  (if (`self.bIsPause Jadge`)
    (set `GameMode_GameOver.bIsPauseJudge` false _output_get)
    (set `self.bIsPause Jadge` false)
    (else
      (set `GameMode_GameOver.bIsPauseJudge` true _output_get)
      (set `self.bIsPause Jadge` true))))

(fn `UserConstructionScript`
  (`parent.UserConstructionScript`))